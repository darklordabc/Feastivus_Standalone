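; BP_ObjectAPI provides Feastivus helper functions for attaching objects to a component socket and detaching them.
; Attach teleports the object to the parent, then snaps its root to the socket's location while keeping world rotation and scale.
; Detach keeps the world transform and can optionally drop the object to the ground using a short downward Visibility trace, without checking that the trace hit.
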(fn FeastivusAttach
  (params (Object :type BP%20Dynamic%20Object%20Object%20Reference) (Parent :type Scene%20Component%20Object%20Reference) (Socket :type Name))
  (Transformation|SetActorLocation Object (Transformation|GetWorldLocation Parent) false true)
  (Transformation|AttachComponentToComponent (Variables|/Script/Engine.Actor|GetRootComponent Object) Parent Socket "SnapToTarget" "KeepWorld" "KeepWorld" true)
  (return Object))

(fn FeastivusDetach
  (params (Object :type BP%20Dynamic%20Object%20Object%20Reference) (Ground :type Boolean))
  (bind _rootcomponent (Variables|/Script/Engine.Actor|GetRootComponent Object))
  (bind _returnvalue (Transformation|GetWorldLocation _rootcomponent))
  (bind _outhit (Collision|LineTraceByChannel 0 _returnvalue (- _returnvalue "0, 0,500.000000") "TraceTypeQuery1" false (Utilities|Array|MakeArray Object 0) "None"))
  (Transformation|DetachFromComponent _rootcomponent "KeepWorld" "KeepWorld" "KeepWorld" true)
  (if Ground
    (Transformation|SetWorldLocation (Variables|/Script/Engine.Actor|GetRootComponent Object) (.Location (Collision|BreakHitResult _outhit)) false true)))